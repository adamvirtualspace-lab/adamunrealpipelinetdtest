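; Actor component that equips its owning character with snow trail triggers, from the DF version of the snow trail system.
; On BeginPlay it prints each of the owner's skeletal meshes with its bone count, then walks their bones.
; Each bone not filtered out by name (root, center, inter, IK, None) gets a runtime-added Child Actor Component spawning BP_DfSpawner, snapped to that bone's location and rotation.
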(event `self.ReceiveBeginPlay`
  (bind _output_get (set `self.Owner` (`self.GetOwner`)))
  (for _array_element (`Actor.K2_GetComponentsByClass` _output_get "/Script/Engine.SkeletalMeshComponent")
    (bind _returnvalue (`SkinnedMeshComponent.GetNumBones` _array_element))
    (`KismetSystemLibrary.PrintString` (`KismetStringLibrary.Concat_StrStr` "Found Skel : " (`KismetSystemLibrary.GetDisplayName` _array_element) " \nWith " (`KismetStringLibrary.Conv_IntToString` _returnvalue) " Bones"))
    (for _index (range (+ _returnvalue 1))
      (bind _returnvalue_2 (`SkinnedMeshComponent.GetBoneName` _array_element _index))
      (bind _returnvalue_3 (`KismetStringLibrary.Conv_NameToString` _returnvalue_2))
      (if (`KismetStringLibrary.Contains` _returnvalue_3 "root")
        _
        (elif (`KismetStringLibrary.Contains` _returnvalue_3 "center")
          _
          (elif (`KismetStringLibrary.Contains` _returnvalue_3 "inter")
            _
            (elif (`KismetStringLibrary.Contains` _returnvalue_3 "ik")
              _
              (elif (not (`KismetStringLibrary.Contains` _returnvalue_3))
                (bind _returnvalue_4 (`|AddComponentByClass` :`self` _output_get :`Class` "/Script/Engine.ChildActorComponent"))
                (`ChildActorComponent.SetChildActorClass` _returnvalue_4 "/Game/Systems/Elementals/SnowTrails/DFVersion/DeformedDF_Sys/BP_DfSpawner.BP_DfSpawner_C")
                (`SceneComponent.K2_AttachToComponent` _returnvalue_4 _array_element _returnvalue_2 "SnapToTarget" "SnapToTarget" "KeepRelative" true)))))))))