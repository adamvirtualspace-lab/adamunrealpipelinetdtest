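; Distance-field spawner for the snow trail deformation system, stamping mesh instances and heavy snow effects where overlaps occur.
; Sphere begin and end overlaps call SpawnDF, which uses name and class checks to skip other DfSpawners and the third-person character.
; It adds an instanced mesh using the spawner's own transform and spawns a Niagara system just below it.
; The instanced mesh component uses absolute location and rotation, detaching it from actor movement.
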(event `self.Sphere.OnComponentEndOverlap`
  (params (OverlappedComponent :type "PrimitiveComponent Object Reference") (OtherActor :type "Actor Object Reference") (OtherComp :type "PrimitiveComponent Object Reference") (OtherBodyIndex :type Integer))
  (bind _returnvalue (`KismetSystemLibrary.GetDisplayName` OtherActor))
  (if (and (not (`KismetStringLibrary.Contains` _returnvalue "DfSpawner")) (!= (`GameplayStatics.GetObjectClass` OtherActor) "/Script/Engine.Character") (not (`KismetStringLibrary.Contains` _returnvalue "character")))
    (`KismetSystemLibrary.PrintString` _returnvalue false false)
    (`self.SpawnDF` OtherActor)))

(event `self.Sphere.OnComponentBeginOverlap`
  (params (OverlappedComponent :type "PrimitiveComponent Object Reference") (OtherActor :type "Actor Object Reference") (OtherComp :type "PrimitiveComponent Object Reference") (OtherBodyIndex :type Integer) (bFromSweep :type Boolean) (SweepResult :type "HitResult Structure (by ref)"))
  (`self.SpawnDF` OtherActor))

(fn `SpawnDF`
  (params (OtherActor :type "Object Object Reference"))
  (bind _returnvalue (`KismetSystemLibrary.GetDisplayName` OtherActor))
  (bind _returnvalue_2 (`self.GetTransform` self))
  (if (`KismetSystemLibrary.IsValid` OtherActor)
    (if (and (not (`KismetStringLibrary.Contains` _returnvalue "DfSpawner")) (!= (`GameplayStatics.GetObjectClass` OtherActor) "/Game/ThirdPerson/Blueprints/BP_ThirdPersonCharacter.BP_ThirdPersonCharacter_C"))
      (`KismetSystemLibrary.PrintString` _returnvalue false false)
      (`|ExecutionSequence`
        (:`then_0`
          (`InstancedStaticMeshComponent.AddInstance` (`self.InstancedStaticMesh`) _returnvalue_2 false))
        (:`then_1`
          (`NiagaraFunctionLibrary.SpawnSystemAtLocation` "/Game/Systems/Elementals/SnowTrails/SnowTrailsAssets/Particles/PSN_SnowHeavy_Surface.PSN_SnowHeavy_Surface" (+ (.location _returnvalue_2) (0.0 0.0 -10.0))))))))

(fn `UserConstructionScript`
  (bind _instancedstaticmesh (`self.InstancedStaticMesh`))
  (set `SceneComponent.bAbsoluteLocation` true _instancedstaticmesh)
  (set `SceneComponent.bAbsoluteRotation` true _instancedstaticmesh)
  (`SceneComponent.SetVisibility` (`self.Sphere`) (`self.Debug`) false))